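; Sliceable fruit actor made of two halves, Half1 and Half2, and a PhysicsConstraint.
; Slice breaks the constraint and throws the halves apart in opposite directions along Half1's right vector.
; Each half gets its own random impulse strength, applied as a velocity change so mass is ignored.
; The event graph and construction script are empty, so nothing in this Blueprint calls Slice.
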(event EventBeginPlay)

(event Collision|EventActorBeginOverlap
  (params (OtherActor :type Actor%20Object%20Reference)))

(event EventTick
  (params (DeltaSeconds :type Float%20%28single-precision%29)))

(fn ConstructionScript)

(fn Slice
  (bind _returnvalue (Math|Random|RandomFloatinRange 3e+02 6e+02))
  (bind _half1 (Variables|Default|GetHalf1))
  (bind _returnvalue_2 (Transformation|GetWorldRotation _half1))
  (bind _returnvalue_3 (Math|Vector|GetRightVector _returnvalue_2))
  (Class|PhysicsConstraintComponent|BreakConstraint (Variables|Default|GetPhysicsConstraint))
  (Physics|AddImpulse _half1 (* _returnvalue_3 (* -1 _returnvalue)) "None" true)
  (Physics|AddImpulse (Variables|Default|GetHalf2) (* _returnvalue_3 _returnvalue) "None" true))