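; SliceFruit is a fruit actor that can be cut once along a plane given by a hit position and normal.
; The construction script copies the Sphere static mesh into a procedural mesh with collision.
; Slice caps the cut with CubeMaterial, then enables physics on the new half and pushes it upward.
; Launch applies randomized linear and spin impulses, but its event-graph call and ten-second destroy are disconnected.
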(event EventBeginPlay)

(fn ConstructionScript
  (Class|KismetProceduralMeshLibrary|CopyProceduralMeshfromStaticMeshComponent (Variables|Default|GetSphere) 0 (Variables|Default|GetProceduralMesh) true))

(fn Slice
  (params (HitPosition :type Vector) (HitNormal :type Vector))
  (if (not (Variables|Default|GetisSliced))
    (Variables|Default|SetisSliced true)
    (bind _outotherhalfprocmesh (Class|KismetProceduralMeshLibrary|SliceProceduralMesh (Variables|Default|GetProceduralMesh) HitPosition HitNormal true "CreateNewSectionForCap" "/Game/Geometry/Meshes/CubeMaterial.CubeMaterial"))
    (Physics|SetSimulatePhysics _outotherhalfprocmesh true)
    (Physics|AddImpulse _outotherhalfprocmesh "0,0.000000,1000.000000" "None" true)))

(fn Launch
  (bind _proceduralmesh (Variables|Default|GetProceduralMesh))
  (Physics|AddImpulse _proceduralmesh (Math|Vector|MakeVector (Math|Random|RandomFloatinRange 4e+02 6e+02) (Math|Random|RandomFloatinRange -1e+02 1e+02) (Math|Random|RandomFloatinRange 9e+02 1.1e+03)) "None" true)
  (Class|PrimitiveComponent|AddAngularImpulseinRadians _proceduralmesh (Math|Vector|MakeVector (Math|Random|RandomFloatinRange -1e+03 1e+03) (Math|Random|RandomFloatinRange -1e+03 1e+03) (Math|Random|RandomFloatinRange -1e+03 1e+03)) "None" true))